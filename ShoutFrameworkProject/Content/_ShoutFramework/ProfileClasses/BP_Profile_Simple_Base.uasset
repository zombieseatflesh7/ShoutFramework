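; Base Blueprint for a simple profile in the Shout framework, which themes a widget with a title and two colors while the profile is selected.
; BeginPlay caches the title and colors from a Profile_Simple_Base data asset.
; Selection applies them to the widget's title, outer icon border and backgrounds.
; Deselection restores a hardcoded "Mission Control" title and default colors before calling the parent.
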(event `self.ReceiveBeginPlay`
  (bind _asprofile_simple_base (cast `/Game/_ShoutFramework/ProfileClasses/Profile_Simple_Base` (`self.Data Asset`)))
  (set `self.Title` (`/Game/_ShoutFramework/ProfileClasses/Profile_Simple_Base.Title` _asprofile_simple_base))
  (set `self.Primary Color` (`/Game/_ShoutFramework/ProfileClasses/Profile_Simple_Base.Primary Color` _asprofile_simple_base))
  (set `self.Secondary Color` (`/Game/_ShoutFramework/ProfileClasses/Profile_Simple_Base.Secondary Color` _asprofile_simple_base)))

(event `self.OnSelected`
  (params (Widget :type "/Game/UI/MissionControl/MissionControl_MainDialogue Object Reference"))
  (bind _title (`/Game/UI/MissionControl/MissionControl_MainDialogue.Title` Widget))
  (bind _returnvalue (`KismetMathLibrary.Conv_ColorToLinearColor` (`self.Primary Color`)))
  (bind _returnvalue_2 (`KismetMathLibrary.Conv_ColorToLinearColor` (`self.Secondary Color`)))
  (`parent.OnSelected` Widget)
  (`TextBlock.SetText` _title (`self.Title`))
  (`TextBlock.SetColorAndOpacity` _title (make `SlateColor` _returnvalue))
  (`Image.SetColorAndOpacity` (`/Game/UI/MissionControl/MissionControl_MainDialogue.IconBorderOuter` Widget) _returnvalue)
  (`Image.SetColorAndOpacity` (`/Game/UI/MissionControl/MissionControl_MainDialogue.BackgroundMain` Widget) _returnvalue_2)
  (`Image.SetColorAndOpacity` (`/Game/UI/MissionControl/MissionControl_MainDialogue.BackgroundTail` Widget) _returnvalue_2))

(event `self.OnDeselected`
  (bind _widget (`self.Widget`))
  (bind _returnvalue (`KismetMathLibrary.Conv_ColorToLinearColor` (make `Color` 21 28 0 179)))
  (bind _returnvalue_2 (`KismetMathLibrary.Conv_ColorToLinearColor` (make `Color` 0 157 255 255)))
  (bind _title (`/Game/UI/MissionControl/MissionControl_MainDialogue.Title` _widget))
  (`TextBlock.SetText` _title "Mission Control")
  (`TextBlock.SetColorAndOpacity` _title (make `SlateColor` _returnvalue_2))
  (`Image.SetColorAndOpacity` (`/Game/UI/MissionControl/MissionControl_MainDialogue.IconBorderOuter` _widget) _returnvalue_2)
  (`Image.SetColorAndOpacity` (`/Game/UI/MissionControl/MissionControl_MainDialogue.BackgroundMain` _widget) _returnvalue)
  (`Image.SetColorAndOpacity` (`/Game/UI/MissionControl/MissionControl_MainDialogue.BackgroundTail` _widget) _returnvalue)
  (`parent.OnDeselected`))

(fn `UserConstructionScript`
  (`parent.UserConstructionScript`))