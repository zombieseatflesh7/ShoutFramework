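; BP_Profile_Simple_Blinking is a Shout Framework profile class that makes a widget's icon blink while selected.
; On BeginPlay it copies the blink image, interval range and duration from its Profile_Simple_Blinking data asset.
; Selection starts a chain of one-shot timers that alternate the normal and blink images, with randomized gaps between blinks.
; Deselection clears the pending timer.
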(event `self.ReceiveBeginPlay`
  (`parent.ReceiveBeginPlay`)
  (bind _asprofile_simple_blinking (cast `/Game/_ShoutFramework/ProfileClasses/Profile_Simple_Blinking` (`self.Data Asset`)))
  (set `self.Icon Blink` (`/Game/_ShoutFramework/ProfileClasses/Profile_Simple_Blinking.Icon Blink` _asprofile_simple_blinking))
  (set `self.Min Time` (`/Game/_ShoutFramework/ProfileClasses/Profile_Simple_Blinking.Min Time` _asprofile_simple_blinking))
  (set `self.Max Time` (`/Game/_ShoutFramework/ProfileClasses/Profile_Simple_Blinking.Max Time` _asprofile_simple_blinking))
  (set `self.Duration` (`/Game/_ShoutFramework/ProfileClasses/Profile_Simple_Blinking.Duration` _asprofile_simple_blinking)))

(event `self.OnSelected`
  (params (Widget :type "/Game/UI/MissionControl/MissionControl_MainDialogue Object Reference"))
  (`parent.OnSelected` Widget)
  (`/Game/UI/_GlobalAssets/MaskedImage/UI_MaskedImage.SetImage` (`/Game/UI/MissionControl/MissionControl_MainDialogue.Icon` Widget) (`self.Icon`) false)
  (bind _returnvalue (`KismetSystemLibrary.K2_SetTimerDelegate` (delegate `Event Blink`) (`KismetMathLibrary.RandomFloatInRange` 0.0 (`self.Max Time`))))
  (set `self.Timer` _returnvalue))

(event `Event Blink`
  (`/Game/UI/_GlobalAssets/MaskedImage/UI_MaskedImage.SetImage` (`/Game/UI/MissionControl/MissionControl_MainDialogue.Icon` (`self.Widget`)) (`self.Icon Blink`) false)
  (bind _returnvalue (`KismetSystemLibrary.K2_SetTimerDelegate` (delegate `Event Blink End`) (`self.Duration`)))
  (set `self.Timer` _returnvalue))

(event `Event Blink End`
  (`/Game/UI/_GlobalAssets/MaskedImage/UI_MaskedImage.SetImage` (`/Game/UI/MissionControl/MissionControl_MainDialogue.Icon` (`self.Widget`)) (`self.Icon`) false)
  (bind _returnvalue (`KismetSystemLibrary.K2_SetTimerDelegate` (delegate `Event Blink`) (`KismetMathLibrary.RandomFloatInRange` (`self.Min Time`) (`self.Max Time`))))
  (set `self.Timer` _returnvalue))

(event `self.OnDeselected`
  (`KismetSystemLibrary.K2_ClearAndInvalidateTimerHandle` (`self.Timer`))
  (`parent.OnDeselected`))

(fn `UserConstructionScript`
  (`parent.UserConstructionScript`))