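; BP_Profile_Simple is a profile class that displays a static icon texture on a widget while the profile is selected.
; On BeginPlay it casts its DataAsset to Profile_Simple_Texture and caches that asset's Icon.
; Selection sets the widget's icon image to the cached texture, and deselection restores the MissionControl character icon.
; Both handlers also call the parent profile's logic.
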(event `self.ReceiveBeginPlay`
  (`parent.ReceiveBeginPlay`)
  (bind _asprofile_simple_texture (cast `/Game/_ShoutFramework/ProfileClasses/Profile_Simple_Texture` (`self.Data Asset`)))
  (set `self.Icon` (`/Game/_ShoutFramework/ProfileClasses/Profile_Simple_Texture.Icon` _asprofile_simple_texture)))

(event `self.OnSelected`
  (params (Widget :type "/Game/UI/MissionControl/MissionControl_MainDialogue Object Reference"))
  (`parent.OnSelected` Widget)
  (`/Game/UI/_GlobalAssets/MaskedImage/UI_MaskedImage.SetImage` (`/Game/UI/MissionControl/MissionControl_MainDialogue.Icon` Widget) (`self.Icon`) false))

(event `self.OnDeselected`
  (`/Game/UI/_GlobalAssets/MaskedImage/UI_MaskedImage.SetImage` (`/Game/UI/MissionControl/MissionControl_MainDialogue.Icon` (`self.Widget`)) "/Game/UI/Art/MainOnScreenHUD/ClassIcon/Characters/Icon_Character_MissionControl.Icon_Character_MissionControl" false)
  (`parent.OnDeselected`))

(fn `UserConstructionScript`
  (`parent.UserConstructionScript`))