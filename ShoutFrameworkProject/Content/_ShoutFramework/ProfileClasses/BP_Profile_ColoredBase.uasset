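; Base profile Blueprint that recolors and retitles a UI widget while the profile is selected.
; On BeginPlay it copies the title and primary and secondary colors from its Profile_ColoredBase data asset.
; Selection applies the title and primary color to the class label, primary to the outer border, and secondary to two images.
; Deselection restores a hardcoded "Mission Control" title and default colors, with both handlers also calling the parent.
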(event `self.ReceiveBeginPlay`
  (bind _asprofile_colored_base (cast `/Game/_ShoutFramework/ProfileClasses/Profile_ColoredBase` (`self.Data Asset`)))
  (set `self.Title` (`/Game/_ShoutFramework/ProfileClasses/Profile_ColoredBase.Title` _asprofile_colored_base))
  (set `self.Primary Color` (`/Game/_ShoutFramework/ProfileClasses/Profile_ColoredBase.Primary Color` _asprofile_colored_base))
  (set `self.Secondary Color` (`/Game/_ShoutFramework/ProfileClasses/Profile_ColoredBase.Secondary Color` _asprofile_colored_base)))

(event `self.OnSelected`
  (params (Widget :type "/Game/UI/MissionControl/MissionControl_MainDialogue Object Reference"))
  (bind _classlabel (`/Game/UI/MissionControl/MissionControl_MainDialogue.ClassLabel` Widget))
  (bind _returnvalue (`KismetMathLibrary.Conv_ColorToLinearColor` (`self.Primary Color`)))
  (bind _returnvalue_2 (`KismetMathLibrary.Conv_ColorToLinearColor` (`self.Secondary Color`)))
  (`parent.OnSelected` Widget)
  (`TextBlock.SetText` _classlabel (`self.Title`))
  (`TextBlock.SetColorAndOpacity` _classlabel (make `SlateColor` _returnvalue))
  (`Image.SetColorAndOpacity` (`/Game/UI/MissionControl/MissionControl_MainDialogue.BorderOuter` Widget) _returnvalue)
  (`Image.SetColorAndOpacity` (`/Game/UI/MissionControl/MissionControl_MainDialogue.Image_108` Widget) _returnvalue_2)
  (`Image.SetColorAndOpacity` (`/Game/UI/MissionControl/MissionControl_MainDialogue.Image_109` Widget) _returnvalue_2))

(event `self.OnDeselected`
  (bind _widget (`self.Widget`))
  (bind _returnvalue (`KismetMathLibrary.Conv_ColorToLinearColor` (make `Color` 21 28 0 179)))
  (bind _returnvalue_2 (`KismetMathLibrary.Conv_ColorToLinearColor` (make `Color` 0 157 255 255)))
  (bind _classlabel (`/Game/UI/MissionControl/MissionControl_MainDialogue.ClassLabel` _widget))
  (`TextBlock.SetText` _classlabel "Mission Control")
  (`TextBlock.SetColorAndOpacity` _classlabel (make `SlateColor` _returnvalue_2))
  (`Image.SetColorAndOpacity` (`/Game/UI/MissionControl/MissionControl_MainDialogue.BorderOuter` _widget) _returnvalue_2)
  (`Image.SetColorAndOpacity` (`/Game/UI/MissionControl/MissionControl_MainDialogue.Image_108` _widget) _returnvalue)
  (`Image.SetColorAndOpacity` (`/Game/UI/MissionControl/MissionControl_MainDialogue.Image_109` _widget) _returnvalue)
  (`parent.OnDeselected`))

(fn `UserConstructionScript`
  (`parent.UserConstructionScript`))