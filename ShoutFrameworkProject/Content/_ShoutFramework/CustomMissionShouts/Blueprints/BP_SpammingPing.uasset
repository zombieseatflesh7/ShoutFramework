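; BP_SpammingPing makes the local player character say a mission shout when pings are spammed.
; Each ping raises a clamped Annoyance meter that decays over time on Tick.
; Once annoyance passes its threshold outside cooldown, a random roll weighted by Annoyingness and current annoyance can fire the shout through the CommunicationComponent.
; A successful shout resets annoyance and starts a timed cooldown.
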(event `self.ReceiveBeginPlay`)

(event `On Ping`
  (bind _output_get (set `self.Annoyance` (`KismetMathLibrary.FClamp` (+ (`self.Annoyance`) (`self.Annoyingness`)) 0.0 2.0)))
  (if (and (> _output_get 1.0) (not (`self.On Cooldown`)))
    (if (<= (`KismetMathLibrary.RandomFloat`) (* (`self.Annoyingness`) (`self.Annoyance`)))
      (`CommunicationComponent.MissionShout` (`PlayerCharacter.CommunicationComponent` (`GameFunctionLibrary.GetLocalPlayerCharacter`)) (`self.Shout`) false)
      (set `self.On Cooldown` true)
      (`KismetSystemLibrary.K2_SetTimerDelegate` (delegate `Cooldown Over`) (`self.Cooldown`))
      (set `self.Annoyance` 0.0))))

(event `Cooldown Over`
  (set `self.On Cooldown` false))

(event `self.ReceiveTick`
  (params (DeltaSeconds :type "Float (single-precision)"))
  (set `self.Annoyance` (`KismetMathLibrary.FClamp` (- (`self.Annoyance`) (* DeltaSeconds (/ 1.0 (`self.Decay Time`)))) 0.0 2.0)))

(fn `UserConstructionScript`)