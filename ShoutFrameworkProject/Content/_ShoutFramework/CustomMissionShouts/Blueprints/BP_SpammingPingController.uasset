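; Server-side controller that triggers shouts when players spam laser-pointer pings on certain targets.
; On BeginPlay it spawns one BP_SpammingPing per category (dwarves, Data Cell, Data Rack, Heartstone, Error Cube), each with its own shout and some with tuned annoyingness or cooldown.
; Tick binds every player character's laser-pointer event each frame, rather than once.
; The handler matches the hit target's class and forwards OnPing to the corresponding spam tracker.
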(event `self.ReceiveBeginPlay`
  (bind _returnvalue (`KismetMathLibrary.MakeTransform` (0.0 0.0 0.0)))
  (if (`KismetSystemLibrary.IsServer`)
    (`|ExecutionSequence`
      (:`then_0`
        (bind _returnvalue_2 (`|SpawnActorFromClass` "/Game/_ShoutFramework/CustomMissionShouts/Blueprints/BP_SpammingPing.BP_SpammingPing_C" _returnvalue "AlwaysSpawn" "OverrideRootScale" null "/Game/_ShoutFramework/CustomMissionShouts/DialogDataAssets/Spamming_Dwarves/DDA_Spamming_Dwarves.DDA_Spamming_Dwarves" 0.05 60.0 60.0 null))
        (set `self.Spamming_Dwarf` _returnvalue_2)
        (bind _returnvalue_3 (`|SpawnActorFromClass` "/Game/_ShoutFramework/CustomMissionShouts/Blueprints/BP_SpammingPing.BP_SpammingPing_C" _returnvalue "AlwaysSpawn" "OverrideRootScale" null "/Game/_ShoutFramework/CustomMissionShouts/DialogDataAssets/Spamming_DataCell/DDA_Spamming_DataCell.DDA_Spamming_DataCell" 0.02 60.0 60.0 null))
        (set `self.Spamming_DataCell` _returnvalue_3)
        (bind _returnvalue_4 (`|SpawnActorFromClass` "/Game/_ShoutFramework/CustomMissionShouts/Blueprints/BP_SpammingPing.BP_SpammingPing_C" _returnvalue "AlwaysSpawn" "OverrideRootScale" null "/Game/_ShoutFramework/CustomMissionShouts/DialogDataAssets/Spamming_ErrorCube/DDA_Spamming_ErrorCube.DDA_Spamming_ErrorCube" 0.02 60.0 60.0 null))
        (set `self.Spamming_ErrorCube` _returnvalue_4)
        (bind _returnvalue_5 (`|SpawnActorFromClass` "/Game/_ShoutFramework/CustomMissionShouts/Blueprints/BP_SpammingPing.BP_SpammingPing_C" _returnvalue "AlwaysSpawn" "OverrideRootScale" null "/Game/_ShoutFramework/CustomMissionShouts/DialogDataAssets/Spamming_DataRack/DDA_Spamming_DataRack.DDA_Spamming_DataRack" 0.05 60.0 30.0 null))
        (set `self.Spamming_DataRack` _returnvalue_5)
        (bind _returnvalue_6 (`|SpawnActorFromClass` "/Game/_ShoutFramework/CustomMissionShouts/Blueprints/BP_SpammingPing.BP_SpammingPing_C" _returnvalue "AlwaysSpawn" "OverrideRootScale" null "/Game/_ShoutFramework/CustomMissionShouts/DialogDataAssets/Spamming_Heartstone/DDA_Spamming_Heartstone.DDA_Spamming_Heartstone" 0.05 60.0 30.0 null))
        (set `self.Spamming_Heartstone` _returnvalue_6))
      (:`then_1`
        (`self.SetActorTickEnabled` true)))))

(event `self.ReceiveTick`
  (params (DeltaSeconds :type "Float (single-precision)"))
  (for _array_element (`ActorFunctionLibrary.GetAllPlayerCharacters`)
    (add `PlayerCharacter.OnLaserPointerEvent` _array_element (delegate `OnLaserPointerEvent_Event_0`))))

(event `OnLaserPointerEvent_Event_0`
  (params (HitInfo :type "LaserPointerTarget Structure (by ref)"))
  (bind _returnvalue (`GameplayStatics.GetObjectClass` (`.Target` (break `LaserPointerTarget` HitInfo))))
  (if (`KismetMathLibrary.ClassIsChildOf` _returnvalue "/Script/FSD.PlayerCharacter")
    (`/Game/_ShoutFramework/CustomMissionShouts/Blueprints/BP_SpammingPing.On Ping` (`self.Spamming_Dwarf`))
    (elif (== _returnvalue "/Game/Critters/Prospector/BP_DataCell.BP_DataCell_C")
      (`/Game/_ShoutFramework/CustomMissionShouts/Blueprints/BP_SpammingPing.On Ping` (`self.Spamming_DataCell`))
      (elif (== _returnvalue "/Game/GameElements/Objectives/Facility/BP_FacilityCore_DataRack.BP_FacilityCore_DataRack_C")
        (`/Game/_ShoutFramework/CustomMissionShouts/Blueprints/BP_SpammingPing.On Ping` (`self.Spamming_DataRack`))
        (elif (== _returnvalue "/Game/GameElements/Resources/Embedded/EscortGem/BP_EscortGem_Heartstone.BP_EscortGem_Heartstone_C")
          (`/Game/_ShoutFramework/CustomMissionShouts/Blueprints/BP_SpammingPing.On Ping` (`self.Spamming_Heartstone`))
          (elif (== _returnvalue "/Game/GameElements/Resources/Embedded/UnknownArtifact/BP_UnknownArtifact.BP_UnknownArtifact_C")
            (`/Game/_ShoutFramework/CustomMissionShouts/Blueprints/BP_SpammingPing.On Ping` (`self.Spamming_ErrorCube`))))))))

(fn `UserConstructionScript`)