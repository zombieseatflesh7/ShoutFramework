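; Shout framework condition class that combines a list of sub-conditions into one boolean using AND, OR or XOR.
; Evaluate casts its parameters to Logical_Condition_GlobalOnly and runs each entry through FrameworkMod's EvaluateCondition.
; AND and OR short-circuit, while XOR flips the result on each true entry, giving an odd-parity check.
; All branches share one exit, which inverts the result when the Not flag is set.
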(event `self.Pre Evaluate`)

(fn `Evaluate`
  (params (Parameters :type "/Game/_ShoutFramework/ConditionClasses/Condition_Base Object Reference"))
  (returns (Result :type Boolean))
  (locals (bool :type Boolean))
  (bind _bool (`local.bool`))
  (bind _aslogical_condition_global_only (cast `/Game/_ShoutFramework/ConditionClasses/Logic/Logical_Condition_GlobalOnly` Parameters))
  (switch `/Game/_ShoutFramework/ConditionClasses/Structs/ELogicOperator` (`/Game/_ShoutFramework/ConditionClasses/Logic/Logical_Condition_GlobalOnly.Operator` _aslogical_condition_global_only)
    (:`NewEnumerator0`
      (bind _conditions (`/Game/_ShoutFramework/ConditionClasses/Logic/Logical_Condition_GlobalOnly.Conditions` _aslogical_condition_global_only))
      (for _array_element _conditions
        (bind _result (`/Game/ShoutFramework/ShoutFrameworkMod.Evaluate Condition` (`self.FrameworkMod`) _array_element))
        (if (not _result)
          (set `local.bool` false)
          (return (select `bool` (`/Game/_ShoutFramework/ConditionClasses/Logic/Logical_Condition_GlobalOnly.Not` _aslogical_condition_global_only) :`false` _bool :`true` (not _bool)))))
      (set `local.bool` true) ; True if all true
    )
    (:`NewEnumerator1`
      (for _array_element_2 _conditions
        (bind _result_2 (`/Game/ShoutFramework/ShoutFrameworkMod.Evaluate Condition` (`self.FrameworkMod`) _array_element_2))
        (if _result_2
          (set `local.bool` true)
          (return (select `bool` (`/Game/_ShoutFramework/ConditionClasses/Logic/Logical_Condition_GlobalOnly.Not` _aslogical_condition_global_only) :`false` _bool :`true` (not _bool)))))
      (set `local.bool` false) ; False if none true
    )
    (:`NewEnumerator2`
      (for _array_element_3 _conditions
        (bind _result_3 (`/Game/ShoutFramework/ShoutFrameworkMod.Evaluate Condition` (`self.FrameworkMod`) _array_element_3))
        (if _result_3
          (set `local.bool` (not (`local.bool`)))))))
  (return (select `bool` (`/Game/_ShoutFramework/ConditionClasses/Logic/Logical_Condition_GlobalOnly.Not` _aslogical_condition_global_only) :`false` _bool :`true` (not _bool))))