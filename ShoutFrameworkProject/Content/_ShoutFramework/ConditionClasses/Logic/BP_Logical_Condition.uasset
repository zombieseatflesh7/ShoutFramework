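; Shout Framework condition class that combines a list of sub-conditions with a logical AND, OR or XOR operator.
; Evaluate casts its parameters to Logical_Condition and runs each entry through FrameworkMod's EvaluateCondition.
; AND and OR short-circuit on the first deciding result, while XOR toggles on every true result, giving odd parity.
; An optional Not flag inverts the final result, which also allows negated forms of each operator.
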(fn `Evaluate`
  (params (Parameters :type "/Game/_ShoutFramework/ConditionClasses/Condition_Base Object Reference"))
  (returns (Result :type Boolean))
  (locals (bool :type Boolean))
  (bind _bool (`local.bool`))
  (bind _aslogical_condition (cast `/Game/_ShoutFramework/ConditionClasses/Logic/Logical_Condition` Parameters))
  (switch `/Game/_ShoutFramework/ConditionClasses/Structs/ELogicOperator` (`/Game/_ShoutFramework/ConditionClasses/Logic/Logical_Condition.Operator` _aslogical_condition)
    (:`NewEnumerator0`
      (bind _conditions (`/Game/_ShoutFramework/ConditionClasses/Logic/Logical_Condition.Conditions` _aslogical_condition))
      (for _array_element _conditions
        (bind _result (`/Game/ShoutFramework/ShoutFrameworkMod.Evaluate Condition` (`self.FrameworkMod`) _array_element))
        (if (not _result)
          (set `local.bool` false)
          (return (select `bool` (`/Game/_ShoutFramework/ConditionClasses/Logic/Logical_Condition.Not` _aslogical_condition) :`false` _bool :`true` (not _bool)))))
      (set `local.bool` true) ; True if all true
    )
    (:`NewEnumerator1`
      (for _array_element_2 _conditions
        (bind _result_2 (`/Game/ShoutFramework/ShoutFrameworkMod.Evaluate Condition` (`self.FrameworkMod`) _array_element_2))
        (if _result_2
          (set `local.bool` true)
          (return (select `bool` (`/Game/_ShoutFramework/ConditionClasses/Logic/Logical_Condition.Not` _aslogical_condition) :`false` _bool :`true` (not _bool)))))
      (set `local.bool` false) ; False if none true
    )
    (:`NewEnumerator2`
      (for _array_element_3 _conditions
        (bind _result_3 (`/Game/ShoutFramework/ShoutFrameworkMod.Evaluate Condition` (`self.FrameworkMod`) _array_element_3))
        (if _result_3
          (set `local.bool` (not (`local.bool`)))))))
  (return (select `bool` (`/Game/_ShoutFramework/ConditionClasses/Logic/Logical_Condition.Not` _aslogical_condition) :`false` _bool :`true` (not _bool))))