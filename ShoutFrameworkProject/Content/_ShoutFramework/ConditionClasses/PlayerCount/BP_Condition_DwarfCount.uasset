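; Shout framework condition that tests how many player characters (dwarves) are in the game.
; PreEvaluate caches the length of the player character list as NumPlayers.
; Evaluate casts its parameters to Condition_DwarfCount and compares the cached number to the configured count using the selected comparison operator.
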(event `/Game/_ShoutFramework/ConditionClasses/BP_Condition_Base.Pre Evaluate`
  (set `self.Num Players` (`KismetArrayLibrary.Array_Length` (`ActorFunctionLibrary.GetAllPlayerCharacters`))))

(fn `Evaluate`
  (params (Parameters :type "/Game/_ShoutFramework/ConditionClasses/Condition_Base Object Reference"))
  (returns (Result :type Boolean))
  (bind _ascondition_dwarf_count (cast `/Game/_ShoutFramework/ConditionClasses/PlayerCount/Condition_DwarfCount` Parameters))
  (return (select `EComparisonMethod` (`/Game/_ShoutFramework/ConditionClasses/PlayerCount/Condition_DwarfCount.Comparison` _ascondition_dwarf_count) :`Equal_To` (== (`self.Num Players`) (`/Game/_ShoutFramework/ConditionClasses/PlayerCount/Condition_DwarfCount.Count` _ascondition_dwarf_count)) :`Not_Equal_To` (!= (`self.Num Players`) (`/Game/_ShoutFramework/ConditionClasses/PlayerCount/Condition_DwarfCount.Count` _ascondition_dwarf_count)) :`Greater_Than_Or_Equal_To` (>= (`self.Num Players`) (`/Game/_ShoutFramework/ConditionClasses/PlayerCount/Condition_DwarfCount.Count` _ascondition_dwarf_count)) :`Less_Than_Or_Equal_To` (<= (`self.Num Players`) (`/Game/_ShoutFramework/ConditionClasses/PlayerCount/Condition_DwarfCount.Count` _ascondition_dwarf_count)) :`Greater_Than` (> (`self.Num Players`) (`/Game/_ShoutFramework/ConditionClasses/PlayerCount/Condition_DwarfCount.Count` _ascondition_dwarf_count)) :`Less_Than` (< (`self.Num Players`) (`/Game/_ShoutFramework/ConditionClasses/PlayerCount/Condition_DwarfCount.Count` _ascondition_dwarf_count)))))