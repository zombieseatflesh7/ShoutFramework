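; Shout framework condition that checks whether the current mission fits allowed Deep Dive types and stages.
; On BeginPlay outside the Space Rig it polls every 0.1 seconds until the generated mission is valid, then caches Deep Dive, Elite and completed-stage state.
; Evaluate tests that state against the Condition_DeepDive parameters: normal or elite plus the current stage, or the non-Deep-Dive flag for other missions and the Space Rig.
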(event `self.ReceiveBeginPlay`
  (bind _returnvalue (`FSDGameInstance.GetGeneratedMission` (`GameFunctionLibrary.GetFSDGameInstance` self)))
  (bind _returnvalue_2 (`DeepDiveFunctionLibrary.GetDeepDiveFromMission` _returnvalue))
  (if (not (`/Game/ShoutFramework/ShoutFrameworkMod.Is On Spacerig` (`self.FrameworkMod`)))
    (`/Engine/EditorBlueprintResources/StandardMacros.IsValid` _returnvalue :!label _label
      (:`Is Valid`
        (bind _output_get (set `self.Is DD` (`GeneratedMission.IsDeepDive` _returnvalue)))
        (if _output_get
          (set `self.Is EDD` (`DeepDiveFunctionLibrary.IsEliteDeepDive` _returnvalue_2))
          (set `self.Stage` (`KismetArrayLibrary.Array_Length` (`DeepDive.StagesCompleted` _returnvalue_2)))))
      (:`Is Not Valid`
        (`KismetSystemLibrary.Delay` 0.1)
        (goto _label)))
    (else
      (set `self.Is DD` false))))

(fn `Evaluate`
  (params (Parameters :type "/Game/_ShoutFramework/ConditionClasses/Condition_Base Object Reference"))
  (returns (Result :type Boolean))
  (bind _ascondition_deep_dive (cast `/Game/_ShoutFramework/ConditionClasses/MissionType/Condition_DeepDive` Parameters))
  (if (`self.Is DD`)
    (return (and (select `bool` (`self.Is EDD`) :`false` (`/Game/_ShoutFramework/ConditionClasses/MissionType/Condition_DeepDive.Normal Deep Dive` _ascondition_deep_dive) :`true` (`/Game/_ShoutFramework/ConditionClasses/MissionType/Condition_DeepDive.Elite Deep Dive` _ascondition_deep_dive)) (select `int` (`self.Stage`) :`0` (`/Game/_ShoutFramework/ConditionClasses/MissionType/Condition_DeepDive.Stage 1` _ascondition_deep_dive) :`1` (`/Game/_ShoutFramework/ConditionClasses/MissionType/Condition_DeepDive.Stage 2` _ascondition_deep_dive) :`2` (`/Game/_ShoutFramework/ConditionClasses/MissionType/Condition_DeepDive.Stage 3` _ascondition_deep_dive)))) ; Allowed on this DD mission
    (else
      (return (`/Game/_ShoutFramework/ConditionClasses/MissionType/Condition_DeepDive.Not Deep Dive` _ascondition_deep_dive)) ; Allowed on normal missions
    )))