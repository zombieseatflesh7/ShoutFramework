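; Custom shout Blueprint that triggers a mission shout when the Drilldozer takes damage during an Escort objective.
; On BeginPlay the server polls each second until the primary objective and its EscortMule exist, then binds to the mule's damage event.
; Each hit rolls a damage-weighted chance and shouts only if health falls within bands inside three normalized ranges and Mission Control is not already speaking.
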(event Custom|OnDozerTakenDamageEvent
  (params (Amount :type Float%20%28single-precision%29))
  (CallFunction|OnDozerTakenDamage Amount))

(event EventBeginPlay
  (bind _returnvalue (Class|GameFunctionLibrary|GetFSDGameMode))
  (bind _objectivesmanager (Variables|/Script/FSD.FSDGameMode|GetObjectivesManager _returnvalue))
  (bind _returnvalue_2 (Class|ObjectivesManager|GetPrimaryObjective _objectivesmanager))
  (if (Networking|IsServer)
    (Utilities|IsValid _returnvalue_2 :!label _label ; Objective doesn't exist at the start of the mission.
      (:Is%20Valid
        (if (Utilities|ClassIsChildOf (Utilities|GetClass _returnvalue_2) "/Script/FSD.EscortObjective")
          (bind _asescort_objective (Utilities|Casting|CastToEscortObjective _returnvalue_2))
          (Utilities|IsValid (Variables|/Script/FSD.EscortObjective|GetEscortMule _asescort_objective) :!label _label_2 ; Dozer doesn't exist at the start of the mission.
            (:Is%20Valid
              (bind _asescort_objective_2 (Utilities|Casting|CastToEscortObjective _returnvalue_2))
              (bind _output_get (Variables|Default|SetDrilldozerRef (Variables|/Script/FSD.EscortObjective|GetEscortMule _asescort_objective_2)))
              (EventDispatchers|AssignOnDamageTaken (Variables|/Script/FSD.EscortMule|GetHealthComponent _output_get) (delegate Custom|OnDozerTakenDamageEvent)))
            (:Is%20Not%20Valid
              (Utilities|FlowControl|Delay 1.0)
              (goto _label_2)))))
      (:Is%20Not%20Valid
        (Utilities|FlowControl|Delay 1.0)
        (goto _label)))))

(fn ConstructionScript)

(fn OnDozerTakenDamage
  (params (amount :type Float%20%28single-precision%29))
  (bind _drilldozerref (Variables|Default|GetDrilldozerRef))
  (bind _healthcomponent (Variables|/Script/FSD.EscortMule|GetHealthComponent _drilldozerref))
  (bind _returnvalue (Class|HealthComponentBase|GetHealthPct _healthcomponent))
  (bind _output_get (LocalVariables|Setchance (Math|Random|RandomBoolwithWeight (Math|Float|Min(Float) (/ amount 5e+01) 1.0))))
  (if (Math|Boolean|ANDBoolean (Math|Boolean|ORBoolean (|((0.400000<x)&&(x<0.980000)) (Math|Float|NormalizetoRange _returnvalue 0.0 0.571429)) (|((0.200000<x)&&(x<0.950000)) (Math|Float|NormalizetoRange _returnvalue 0.571429 0.785714)) (|((0.200000<x)&&(x<0.950000)) (Math|Float|NormalizetoRange _returnvalue 0.785714 1.0))) _output_get (not (Class|CommunicationComponent|IsMissionControlSpeaking (Variables|/Script/FSD.PlayerCharacter|GetCommunicationComponent (Class|GameFunctionLibrary|GetLocalPlayerCharacter)))))
    (Class|CommunicationComponent|MissionShout "/Game/ShoutFramework/CustomShouts/DataAssets/DDA_Escort_DrilldozerTakingDamage.DDA_Escort_DrilldozerTakingDamage" false)))