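; Shout framework condition that tests how intoxicated a dwarf is against a configured threshold.
; PreEvaluate caches the target percent from the dwarf's IntoxicationComponent.
; Evaluate casts its parameters to Condition_Intoxication and compares the cached value using the chosen greater-than-or-equal or less-than operator.
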(event `/Game/_ShoutFramework/ConditionBase/BP_Condition_Base.Pre Evaluate`
  (set `self.Percent` (`.TargetPercent` (break `LerpingPercent` (`CharacterIntoxicationComponent.IntoxicationPercent` (`PlayerCharacter.IntoxicationComponent` (`self.Dwarf`)))))))

(fn `Evaluate`
  (params (Parameters :type "/Game/_ShoutFramework/ConditionBase/Condition_Base Object Reference"))
  (returns (Result :type Boolean))
  (bind _ascondition_intoxication (cast `/Game/ShoutMods/ShoutFramework/ConditionClasses/Dwarfs/Condition_Intoxication` Parameters))
  (return (select `/Game/ShoutMods/ShoutFramework/ConditionClasses/Structs/EGreaterthanLessthan` (`/Game/ShoutMods/ShoutFramework/ConditionClasses/Dwarfs/Condition_Intoxication.Comparison` _ascondition_intoxication) :`NewEnumerator0` (>= (`self.Percent`) (`/Game/ShoutMods/ShoutFramework/ConditionClasses/Dwarfs/Condition_Intoxication.Percent` _ascondition_intoxication)) :`NewEnumerator1` (< (`self.Percent`) (`/Game/ShoutMods/ShoutFramework/ConditionClasses/Dwarfs/Condition_Intoxication.Percent` _ascondition_intoxication)))))