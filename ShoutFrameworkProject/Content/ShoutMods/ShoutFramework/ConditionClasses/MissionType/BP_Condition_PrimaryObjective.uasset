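; BP_Condition_PrimaryObjective is a Shout Framework condition that checks whether the current mission's primary objective matches the one given in its parameters.
; On BeginPlay it polls every 0.1 seconds until the generated mission is valid, then maps the objective asset to an enum and caches it.
; On the Space Rig it caches the same fallback value used for unrecognized objectives.
; Evaluate compares the cached value against the condition parameters.
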(event `self.ReceiveBeginPlay`
  (bind _returnvalue (`FSDGameInstance.GetGeneratedMission` (`GameFunctionLibrary.GetFSDGameInstance` self)))
  (if (not (`/Game/ShoutFramework/ShoutFrameworkMod.Is On Spacerig` (`self.FrameworkMod`)))
    (`/Engine/EditorBlueprintResources/StandardMacros.IsValid` _returnvalue :!label _label
      (:`Is Valid`
        (set `self.Primary Objective` (`self.Get Primary Objective` _returnvalue)))
      (:`Is Not Valid`
        (`KismetSystemLibrary.Delay` 0.1)
        (goto _label)))
    (else
      (set `self.Primary Objective` "NewEnumerator8") ; If on spacerig
    )))

(fn `Evaluate`
  (params (Parameters :type "/Game/_ShoutFramework/ConditionBase/Condition_Base Object Reference"))
  (returns (Result :type Boolean))
  (bind _ascondition_primary_objective (cast `/Game/ShoutMods/ShoutFramework/ConditionClasses/MissionType/Condition_PrimaryObjective` Parameters))
  (return (`|EnumEquality` (`self.Primary Objective`) (`/Game/ShoutMods/ShoutFramework/ConditionClasses/MissionType/Condition_PrimaryObjective.Primary Objective` _ascondition_primary_objective))))

(fn `Get Primary Objective`
  (params (Mission :type "GeneratedMission Object Reference"))
  (returns (Enum :type "/Game/ShoutMods/ShoutFramework/ConditionClasses/Structs/EPrimaryObjective Enum"))
  (bind _primaryobjective (`GeneratedMission.PrimaryObjective` Mission))
  (if (== _primaryobjective "/Game/GameElements/Objectives/OBJ_1st_Extraction.OBJ_1st_Extraction_C")
    (return "NewEnumerator0")
    (elif (== _primaryobjective "/Game/GameElements/Objectives/OBJ_1st_Gather_AlienEggs.OBJ_1st_Gather_AlienEggs_C")
      (return "NewEnumerator1")
      (elif (== _primaryobjective "/Game/GameElements/Objectives/Elimination/OBJ_Eliminate_Eggs.OBJ_Eliminate_Eggs_C")
        (return "NewEnumerator6")
        (elif (== _primaryobjective "/Game/GameElements/Objectives/OBJ_1st_PointExtraction.OBJ_1st_PointExtraction_C")
          (return "NewEnumerator4")
          (elif (== _primaryobjective "/Game/GameElements/Objectives/Salvage/OBJ_1st_Salvage.OBJ_1st_Salvage_C")
            (return "NewEnumerator3")
            (elif (== _primaryobjective "/Game/GameElements/Objectives/Escort/OBJ_1st_Escort.OBJ_1st_Escort_C")
              (return "NewEnumerator5")
              (elif (== _primaryobjective "/Game/GameElements/Objectives/Refinery/OBJ_1st_Refinery.OBJ_1st_Refinery_C")
                (return "NewEnumerator2")
                (elif (== _primaryobjective "/Game/GameElements/Objectives/Facility/OBJ_1st_Facility.OBJ_1st_Facility_C")
                  (return "NewEnumerator7")
                  (else
                    (return "NewEnumerator8")))))))))))