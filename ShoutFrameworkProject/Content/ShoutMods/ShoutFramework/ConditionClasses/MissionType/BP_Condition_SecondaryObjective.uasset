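; Shout framework condition that checks whether the current mission's secondary objective matches the one in the supplied condition parameters.
; On BeginPlay it retries every 0.1 seconds until the generated mission is valid, then maps its first secondary objective, standard or Deep Dive, to an enum.
; The Space Rig and unrecognised objectives share one fallback value.
; Evaluate compares the cached value with the parameter.
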(event `self.ReceiveBeginPlay`
  (bind _returnvalue (`FSDGameInstance.GetGeneratedMission` (`GameFunctionLibrary.GetFSDGameInstance` self)))
  (if (not (`/Game/ShoutFramework/ShoutFrameworkMod.Is On Spacerig` (`self.FrameworkMod`)))
    (`/Engine/EditorBlueprintResources/StandardMacros.IsValid` _returnvalue :!label _label
      (:`Is Valid`
        (set `self.Secondary Objective` (`self.Get Secondary Objective` (`|GetArrayItem` (`GeneratedMission.SecondaryObjectives` _returnvalue)))))
      (:`Is Not Valid`
        (`KismetSystemLibrary.Delay` 0.1)
        (goto _label)))
    (else
      (set `self.Secondary Objective` "NewEnumerator8") ; Is on spacerig
    )))

(fn `Evaluate`
  (params (Parameters :type "/Game/_ShoutFramework/ConditionBase/Condition_Base Object Reference"))
  (returns (Result :type Boolean))
  (bind _ascondition_secondary_objective (cast `/Game/ShoutMods/ShoutFramework/ConditionClasses/MissionType/Condition_SecondaryObjective` Parameters))
  (return (`|EnumEquality` (`self.Secondary Objective`) (`/Game/ShoutMods/ShoutFramework/ConditionClasses/MissionType/Condition_SecondaryObjective.Secondary Objective` _ascondition_secondary_objective))))

(fn `Get Secondary Objective`
  (params (Objective :type "Objective Class Reference"))
  (returns (Enum :type "/Game/ShoutMods/ShoutFramework/ConditionClasses/Structs/ESecondaryObjective Enum"))
  (if (== Objective "/Game/GameElements/Objectives/OBJ_2nd_Find_Fossil.OBJ_2nd_Find_Fossil_C")
    (return "NewEnumerator0")
    (elif (== Objective "/Game/GameElements/Objectives/OBJ_2nd_Find_ApocaBloom.OBJ_2nd_Find_ApocaBloom_C")
      (return "NewEnumerator1")
      (elif (== Objective "/Game/GameElements/Objectives/OBJ_2nd_Find_BooloCap.OBJ_2nd_Find_BooloCap_C")
        (return "NewEnumerator2")
        (elif (== Objective "/Game/GameElements/Objectives/OBJ_2nd_Mine_Dystrum.OBJ_2nd_Mine_Dystrum_C")
          (return "NewEnumerator3")
          (elif (== Objective "/Game/GameElements/Objectives/OBJ_2nd_Find_Ebonut.OBJ_2nd_Find_Ebonut_C")
            (return "NewEnumerator4")
            (elif (== Objective "/Game/GameElements/Objectives/OBJ_2nd_KillFleas.OBJ_2nd_KillFleas_C")
              (return "NewEnumerator5")
              (elif (== Objective "/Game/GameElements/Objectives/OBJ_2nd_Find_Gunkseed.OBJ_2nd_Find_Gunkseed_C")
                (return "NewEnumerator6")
                (elif (== Objective "/Game/GameElements/Objectives/OBJ_2nd_Mine_Hollomite.OBJ_2nd_Mine_Hollomite_C")
                  (return "NewEnumerator7")
                  (elif (== Objective "/Game/GameElements/Objectives/DeepDive/OBJ_DD_Morkite.OBJ_DD_Morkite_C")
                    (return "NewEnumerator9")
                    (elif (== Objective "/Game/GameElements/Objectives/DeepDive/OBJ_DD_AlienEggs.OBJ_DD_AlienEggs_C")
                      (return "NewEnumerator10")
                      (elif (== Objective "/Game/GameElements/Objectives/DeepDive/OBJ_DD_Elimination_Eggs.OBJ_DD_Elimination_Eggs_C")
                        (return "NewEnumerator11")
                        (elif (== Objective "/Game/GameElements/Objectives/DeepDive/Reparation/OBJ_DD_RepairMinimules.OBJ_DD_RepairMinimules_C")
                          (return "NewEnumerator12")
                          (elif (== Objective "/Game/GameElements/Objectives/DeepDive/Defense/OBJ_DD_Defense.OBJ_DD_Defense_C")
                            (return "NewEnumerator13")
                            (else
                              (return "NewEnumerator8"))))))))))))))))