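; Shout Framework condition that checks whether the current Deep Rock Galactic mission's biome matches a configured biome.
; On BeginPlay it polls every 0.1 seconds until the generated mission's biome is valid, then maps the biome index to an enum and caches it.
; On the space rig it caches a dedicated enum value instead.
; Evaluate casts its parameters to Condition_Biome and compares that biome to the cached one.
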(event `self.ReceiveBeginPlay`
  (bind _biome (`GeneratedMission.Biome` (`FSDGameInstance.GetGeneratedMission` (`GameFunctionLibrary.GetFSDGameInstance` self))))
  (if (not (`/Game/ShoutFramework/ShoutFrameworkMod.Is On Spacerig` (`self.FrameworkMod`)))
    (`/Engine/EditorBlueprintResources/StandardMacros.IsValid` _biome :!label _label
      (:`Is Valid`
        (set `self.Biome` (`self.Get Biome Enum` _biome)))
      (:`Is Not Valid`
        (`KismetSystemLibrary.Delay` 0.1)
        (goto _label)))
    (else
      (set `self.Biome` "NewEnumerator11") ; Is on spacerig
    )))

(fn `Evaluate`
  (params (Parameters :type "/Game/_ShoutFramework/ConditionBase/Condition_Base Object Reference"))
  (returns (Result :type Boolean))
  (bind _ascondition_biome (cast `/Game/ShoutMods/ShoutFramework/ConditionClasses/MissionType/Condition_Biome` Parameters))
  (return (`|EnumEquality` (`self.Biome`) (`/Game/ShoutMods/ShoutFramework/ConditionClasses/MissionType/Condition_Biome.Biome` _ascondition_biome))))

(fn `Get Biome Enum`
  (params (`Biome Object` :type "Biome Object Reference"))
  (returns (Enum :type "/Game/ShoutMods/ShoutFramework/ConditionClasses/Structs/EBiome Enum"))
  (switch `int` (`Biome.GetBiomeIndex` `Biome Object`)
    (:`0`
      (return "NewEnumerator1"))
    (:`1`
      (return "NewEnumerator2"))
    (:`2`
      (return "NewEnumerator5"))
    (:`3`
      (return "NewEnumerator4"))
    (:`4`
      (return "NewEnumerator8"))
    (:`5`
      (return "NewEnumerator3"))
    (:`6`
      (return "NewEnumerator0"))
    (:`7`
      (return "NewEnumerator9"))
    (:`9`
      (return "NewEnumerator7"))
    (:`10`
      (return "NewEnumerator6"))))