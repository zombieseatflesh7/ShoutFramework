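; Shout Framework condition that tests how many players of a given dwarf class (Driller, Engineer, Gunner or Scout) are present.
; PreEvaluate resets and recounts the four class tallies from all player characters.
; Evaluate casts its parameters to Condition_ClassCount, picks the tally for the requested class and compares it to the target count using the chosen comparison operator.
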(event `/Game/_ShoutFramework/ConditionBase/BP_Condition_Base.Pre Evaluate`
  (set `self.Drillers` 0)
  (set `self.Engineers` 0)
  (set `self.Gunners` 0)
  (set `self.Scouts` 0)
  (for _array_element (`ActorFunctionLibrary.GetAllPlayerCharacters`)
    (bind _class (`/Game/_ShoutFramework/ShoutFrameworkFunctions.GetDwarfClass` _array_element))
    (switch `/Game/ShoutMods/ShoutFramework/ConditionClasses/Structs/EClass` _class
      (:`NewEnumerator0`
        (`/Engine/EditorBlueprintResources/StandardMacros.IncrementInt` (`self.Drillers`)))
      (:`NewEnumerator1`
        (`/Engine/EditorBlueprintResources/StandardMacros.IncrementInt` (`self.Engineers`)))
      (:`NewEnumerator2`
        (`/Engine/EditorBlueprintResources/StandardMacros.IncrementInt` (`self.Gunners`)))
      (:`NewEnumerator3`
        (`/Engine/EditorBlueprintResources/StandardMacros.IncrementInt` (`self.Scouts`))))))

(fn `Evaluate`
  (params (Parameters :type "/Game/_ShoutFramework/ConditionBase/Condition_Base Object Reference"))
  (returns (Result :type Boolean))
  (bind _ascondition_class_count (cast `/Game/ShoutMods/ShoutFramework/ConditionClasses/PlayerCount/Condition_ClassCount` Parameters))
  (bind _returnvalue (select `/Game/ShoutMods/ShoutFramework/ConditionClasses/Structs/EClass` (`/Game/ShoutMods/ShoutFramework/ConditionClasses/PlayerCount/Condition_ClassCount.Class` _ascondition_class_count) :`NewEnumerator0` (`self.Drillers`) :`NewEnumerator1` (`self.Engineers`) :`NewEnumerator2` (`self.Gunners`) :`NewEnumerator3` (`self.Scouts`)))
  (bind _count (`/Game/ShoutMods/ShoutFramework/ConditionClasses/PlayerCount/Condition_ClassCount.Count` _ascondition_class_count))
  (return (select `EComparisonMethod` (`/Game/ShoutMods/ShoutFramework/ConditionClasses/PlayerCount/Condition_ClassCount.Comparison` _ascondition_class_count) :`Equal_To` (== _returnvalue _count) :`Not_Equal_To` (!= _returnvalue _count) :`Greater_Than_Or_Equal_To` (>= _returnvalue _count) :`Less_Than_Or_Equal_To` (<= _returnvalue _count) :`Greater_Than` (> _returnvalue _count) :`Less_Than` (< _returnvalue _count))))