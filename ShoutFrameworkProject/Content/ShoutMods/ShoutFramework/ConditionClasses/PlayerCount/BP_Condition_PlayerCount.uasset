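; Shout framework condition that tests how many player characters are currently in the game.
; PreEvaluate caches the count of all player characters in NumPlayers before evaluation runs.
; Evaluate casts the parameters to Condition_PlayerCount and compares NumPlayers against its Count using the selected comparison operator.
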(event `/Game/_ShoutFramework/ConditionBase/BP_Condition_Base.Pre Evaluate`
  (set `self.Num Players` (`KismetArrayLibrary.Array_Length` (`ActorFunctionLibrary.GetAllPlayerCharacters`))))

(fn `Evaluate`
  (params (Parameters :type "/Game/_ShoutFramework/ConditionBase/Condition_Base Object Reference"))
  (returns (Result :type Boolean))
  (bind _ascondition_player_count (cast `/Game/ShoutMods/ShoutFramework/ConditionClasses/PlayerCount/Condition_PlayerCount` Parameters))
  (return (select `EComparisonMethod` (`/Game/ShoutMods/ShoutFramework/ConditionClasses/PlayerCount/Condition_PlayerCount.Comparison` _ascondition_player_count) :`Equal_To` (== (`self.Num Players`) (`/Game/ShoutMods/ShoutFramework/ConditionClasses/PlayerCount/Condition_PlayerCount.Count` _ascondition_player_count)) :`Not_Equal_To` (!= (`self.Num Players`) (`/Game/ShoutMods/ShoutFramework/ConditionClasses/PlayerCount/Condition_PlayerCount.Count` _ascondition_player_count)) :`Greater_Than_Or_Equal_To` (>= (`self.Num Players`) (`/Game/ShoutMods/ShoutFramework/ConditionClasses/PlayerCount/Condition_PlayerCount.Count` _ascondition_player_count)) :`Less_Than_Or_Equal_To` (<= (`self.Num Players`) (`/Game/ShoutMods/ShoutFramework/ConditionClasses/PlayerCount/Condition_PlayerCount.Count` _ascondition_player_count)) :`Greater_Than` (> (`self.Num Players`) (`/Game/ShoutMods/ShoutFramework/ConditionClasses/PlayerCount/Condition_PlayerCount.Count` _ascondition_player_count)) :`Less_Than` (< (`self.Num Players`) (`/Game/ShoutMods/ShoutFramework/ConditionClasses/PlayerCount/Condition_PlayerCount.Count` _ascondition_player_count)))))