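; Shout framework condition that checks whether a dwarf is of a given player class.
; PreEvaluate maps the Dwarf's character Blueprint (Driller, Engineer, Gunner or Navigator) to a class enum and caches it.
; Evaluate casts the parameters to Condition_PlayerClass and compares the requested class to the cached one.
; Mapping uses exact class equality, so any unmatched character falls back to the Navigator value.
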(event `/Game/_ShoutFramework/BaseClasses/Condition_Base/Condition_Base_Actor.Pre Evaluate`
  (bind _class (`self.GetDwarfClass` (`self.Dwarf`)))
  (set `self.Class` _class))

(fn `Evaluate`
  (params (Parameters :type "/Game/_ShoutFramework/BaseClasses/Condition_Base/Condition_Base Object Reference"))
  (returns (Result :type Boolean))
  (bind _ascondition_player_class (cast `/Game/ShoutMods/ShoutFrameworkContent/ConditionClasses/Dwarfs/Condition_PlayerClass` Parameters))
  (return (`|EnumEquality` (`self.Class`) (`/Game/ShoutMods/ShoutFrameworkContent/ConditionClasses/Dwarfs/Condition_PlayerClass.Class` _ascondition_player_class))))

(fn `GetDwarfClass`
  (params (Dwarf :type "PlayerCharacter Object Reference"))
  (returns (Class :type "/Game/ShoutMods/ShoutFrameworkContent/ConditionClasses/Structs/EClass Enum"))
  (bind _returnvalue (`GameplayStatics.GetObjectClass` Dwarf))
  (if (== _returnvalue "/Game/Character/BP_DrillerCharacter.BP_DrillerCharacter_C")
    (return "NewEnumerator0")
    (elif (== _returnvalue "/Game/Character/BP_EngineerCharacter.BP_EngineerCharacter_C")
      (return "NewEnumerator1")
      (elif (== _returnvalue "/Game/Character/BP_GunnerCharacter.BP_GunnerCharacter_C")
        (return "NewEnumerator2")
        (elif (== _returnvalue "/Game/Character/BP_NavigatorCharacter.BP_NavigatorCharacter_C")
          (return "NewEnumerator3")
          (else
            (return "NewEnumerator3")))))))