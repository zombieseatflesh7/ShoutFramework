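; Uplink variant of a salvage objective point with defense start, complete and fail events, built on a parent class.
; BeginPlay, the construction script and the three defense events only forward to the parent implementation.
; Terrain scanner mesh update, repair cheat and photosensitivity handling are empty stubs, so this graph adds no logic of its own.
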(event `self.ReceiveBeginPlay`
  (`parent.ReceiveBeginPlay`))

(event `/Game/GameElements/Objectives/Salvage/BP_Salvage_Point.OnDefenseStart`
  (`parent.OnDefenseStart`))

(event `/Game/GameElements/Objectives/Salvage/BP_Salvage_Point.OnDefenseComplete`
  (`parent.OnDefenseComplete`))

(event `/Game/GameElements/Objectives/Salvage/BP_Salvage_Point.OnDefenseFail`
  (`parent.OnDefenseFail`))

(event `UpdateTerrainScannerMesh`)

(event `Cheat_RepairUplink`)

(fn `HandlePhotosensitivity`)

(fn `UserConstructionScript`
  (`parent.UserConstructionScript`))