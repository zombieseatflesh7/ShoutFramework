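; BP_CaretakerMortarAction is an action Blueprint for the Caretaker facility objective, named for a mortar attack but currently a skeleton.
; Its start, trigger and stop events and its start-duration estimate only defer to the parent class.
; FireMortar, FireBurst, All_ShowPhaseBombLaunch and LaunchProjectile are empty stubs, so this file holds no firing or projectile logic of its own.
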(event `self.OnStarted`
  (`parent.OnStarted`))

(event `FireMortar`)

(event `self.OnTriggered`
  (`parent.OnTriggered`))

(event `self.OnStopped`
  (`parent.OnStopped`))

(event `FireBurst`)

(event `All_ShowPhaseBombLaunch`
  (params (AttachPointName :type Name)))

(fn `GetEstimatedStartDuration`
  (returns (StartDuration :type "Float (double-precision)"))
  (bind _startduration (`parent.GetEstimatedStartDuration`))
  (return _startduration))

(fn `LaunchProjectile`
  (params (TargetLocation :type "Vector Structure")))