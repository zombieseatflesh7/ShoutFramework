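; Data Vault main facility objective Blueprint, largely a skeleton with no gameplay logic of its own.
; BeginPlay, activation, generators-ready and shield-disable events only forward to their parent implementations.
; Graphs for the Caretaker final fight, tentacle attacks, drones, hatch and cheats are empty stubs or return nothing.
; The alive-players trigger check always returns false.
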(event `self.ReceiveBeginPlay`
  (`parent.ReceiveBeginPlay`))

(event `FadeShield__FinishedFunc`)

(event `FadeShield__UpdateFunc`)

(event `Cheat_TeleportPlayer`)

(event `self.OnActivated`
  (`parent.OnActivated`))

(event `self.OnGeneratorsReady`
  (`parent.OnGeneratorsReady`))

(event `StartFinalFight`)

(event `FinalFightOver`)

(event `RegrowTentacles`)

(event `TryElectricAttack`)

(event `DroneSpawned`
  (params (enemy :type "Pawn Object Reference")))

(event `CaretakerDefeated`
  (params (HealthComponent :type "HealthComponentBase Object Reference")))

(event `OnCaretakerSpawned`
  (params (caretaker :type "/Game/GameElements/Objectives/Facility/Caretaker/ENE_FacilityCaretaker Object Reference")))

(event `self.DisableShields`
  (`parent.DisableShields`))

(event `OnBatteriesExtracted`)

(event `Cheat_DisableShieldEmitter`)

(event `LeftCharged`
  (params (Generator :type "/Game/GameElements/Objectives/Facility/ShieldGenerator/BP_Facility_PowerStation_GeneratorBase Object Reference")))

(event `RightCharged`
  (params (Generator :type "/Game/GameElements/Objectives/Facility/ShieldGenerator/BP_Facility_PowerStation_GeneratorBase Object Reference")))

(event `PreventSpawning`)

(event `KillTentacles`)

(event `PauseTentacles`
  (params (Duration :type "Float (double-precision)")))

(event `OnPause`
  (params (Duration :type "Float (double-precision)")))

(event `CarveOutVault`)

(fn `ActivatorEnganged`)

(fn `AnyAlivePlayersInTrigger`
  (returns (Result :type Boolean))
  (return false))

(fn `BouncePlayer`
  (params (InActor :type "Actor Object Reference") (InHit :type "HitResult Structure")))

(fn `Disable Shield`)

(fn `FadeInLightBelow`)

(fn `FindClosestWeakspotLocation`
  (params (TargetLocaton :type "Vector Structure"))
  (returns (ClosestWeakpointTransform :type "Transform Structure"))
  (return))

(fn `FindValidRangedTarget`
  (params (TentacleRef :type "/Game/GameElements/Objectives/Facility/DefensiveTentacles/ENE_FacilityTentacle Object Reference") (MinDistance :type "Float (double-precision)") (NeedLoS :type Boolean))
  (returns (TargetPlayer :type "Actor Object Reference"))
  (return null))

(fn `GetRandomTentacle`
  (return))

(fn `GetTentacles`
  (return))

(fn `GetTentacleSpawners`
  (return))

(fn `OnRep_Caretaker`)

(fn `OnRep_ChangingFaze`)

(fn `OnRep_Found`)

(fn `OnRep_HasActivated`)

(fn `Open Hatch`)

(fn `SetActivationsRequired`
  (params (activations :type Integer)))

(fn `Setup Patrol Drone`
  (params (drone :type "PatrolBot Object Reference")))

(fn `TryStartMeleeAttack`)

(fn `UpdateLookAtShouts`)

(fn `UserConstructionScript`)