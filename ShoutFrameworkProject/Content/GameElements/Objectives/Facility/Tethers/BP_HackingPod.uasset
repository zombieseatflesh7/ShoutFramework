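; Hacking pod Blueprint for the Facility objective, a drop pod that declares hooks for tethers, hacking state, screens, item dispensing and targeting.
; BeginPlay, the drop and impact events, and state enter/exit only forward to the parent implementation.
; All other events and functions, including effects, salutes, player tracking and targeting queries, are empty or return defaults, so the file holds no logic of its own.
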(event `self.ReceiveBeginPlay`
  (`parent.ReceiveBeginPlay`))

(event `self.ShowDamageEffects`
  (params (Particles :type "ParticleSystem Object Reference") (Location :type "Vector Structure") (Orientation :type "Rotator Structure")))

(event `self.OnDroppodImpact`
  (`parent.OnDroppodImpact`))

(event `SetLightColor`
  (params (Index :type Integer)))

(event `ManageOutlines`)

(event `self.OnDropStarted`
  (`parent.OnDropStarted`))

(event `DeployAnimations`)

(event `self.OnDroppodCloseToImpact`
  (`parent.OnDroppodCloseToImpact`))

(event `ResizeCarver`)

(event `UpdateUseIcon`)

(event `StartFanColoring`)

(event `TakeOff`)

(event `OnBoscoSalute_Event_0`
  (params (ShoutingPlayer :type "PlayerCharacter Object Reference")))

(event `All_Pet`)

(event `self.OnEnterState`
  (params (NextState :type "EHackingPodState Enum" :default "EClosed"))
  (`parent.OnEnterState` NextState))

(event `self.OnExitState`
  (params (oldState :type "EHackingPodState Enum" :default "EClosed"))
  (`parent.OnExitState` oldState))

(event `All_PlaySalute`
  (params (Saluter :type "Actor Object Reference")))

(event `ItemTaken`
  (params (spawnedItem :type "Actor Object Reference")))

(event `OnPlayerJoined_Event_0`
  (params (PlayerState :type "FSDPlayerState Object Reference")))

(event `OnPlayerLeave_Event_0`
  (params (PlayerState :type "FSDPlayerState Object Reference")))

(fn `EnableScreens`
  (params (ScreensActive :type Boolean)))

(fn `FanColorsIntact`
  (returns (FansIntact :type Boolean))
  (return false))

(fn `GetDispenser`
  (return))

(fn `GetIgnoreTethers`
  (returns (ChildTethers :type "Array of Actor Object Reference"))
  (return))

(fn `GetIsTargetable`
  (returns (ReturnValue :type Boolean))
  (return false))

(fn `GetTargetCenterMass`
  (returns (ReturnValue :type "Vector Structure"))
  (return (0.0 0.0 0.0)))

(fn `GetTargetHealthComponent`
  (returns (ReturnValue :type "HealthComponentBase Object Reference"))
  (return null))

(fn `HackingInProgress`
  (returns (NewParam :type Boolean))
  (return false))

(fn `ReconnectTethers`)

(fn `SetShowRange`
  (params (ShowRange :type Boolean)))

(fn `UpdatePlayerCount`)

(fn `UserConstructionScript`)