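; Dialogue profile that replaces the standard widget with an Undertale-style typewriter text box, configured from a Profile_Undertale data asset.
; Selection toggles between the two widgets.
; On play, it drops the incoming audio's pitch and volume to near zero, then stops it when typing finishes.
; Text is split into sentences, word-wrapped to a character limit and padded to keep sentences within three-line pages where possible.
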(event `self.ReceiveBeginPlay`
  (bind _asprofile_undertale (cast `/Game/_TestMod/Undertale/Profile_Undertale` (`self.Data Asset`)))
  (set `self.Character Limit` (`/Game/_TestMod/Undertale/Profile_Undertale.Character Limit` _asprofile_undertale))
  (bind _returnvalue (`|CreateWidget` "/Game/_TestMod/Undertale/UndertaleWidget.UndertaleWidget_C" null (`/Game/_TestMod/Undertale/Profile_Undertale.Font` _asprofile_undertale) (`/Game/_TestMod/Undertale/Profile_Undertale.Line Gap` _asprofile_undertale) (`/Game/_TestMod/Undertale/Profile_Undertale.Typing Speed` _asprofile_undertale) (`/Game/_TestMod/Undertale/Profile_Undertale.Text SFX` _asprofile_undertale) (`/Game/_TestMod/Undertale/Profile_Undertale.Voice Punctuation` _asprofile_undertale)))
  (bind _output_get (set `self.Undertale Widget` _returnvalue))
  (`Image.SetBrushFromTexture` (`/Game/_TestMod/Undertale/UndertaleWidget.CharacterIcon` _output_get) (`/Game/_TestMod/Undertale/Profile_Undertale.Character Icon` _asprofile_undertale) false)
  (add `/Game/_TestMod/Undertale/UndertaleWidget.On Finished` _output_get (delegate `On Finished`))
  (`Widget.SetVisibility` _output_get "Collapsed"))

(event `On Finished`
  (`AudioComponent.Stop` (`self.Audio`)))

(event `self.On Play`
  (params (Audio :type "AudioComponent Object Reference") (Text :type Text))
  (bind _output_get (set `self.Audio` Audio))
  (`AudioComponent.SetPitchMultiplier` _output_get 0.0001)
  (`AudioComponent.SetVolumeMultiplier` _output_get 0.001)
  (`/Game/_TestMod/Undertale/UndertaleWidget.Run Text` (`self.Undertale Widget`) (`self.Format String Into Lines` (`KismetStringLibrary.TrimTrailing` (`KismetStringLibrary.Trim` (`KismetTextLibrary.Conv_TextToString` Text))))))

(event `self.OnSelected`
  (params (Widget :type "/Game/UI/MissionControl/MissionControl_MainDialogue Object Reference"))
  (bind _undertale_widget (`self.Undertale Widget`))
  (`parent.OnSelected` Widget)
  (`Widget.SetVisibility` (`/Game/UI/MissionControl/MissionControl_MainDialogue.MasterBox` (`self.Widget`)) "Collapsed")
  (`Widget.SetVisibility` (`self.Undertale Widget`) "HitTestInvisible")
  (if (not (`Widget.IsInViewport` _undertale_widget))
    (`UserWidget.AddToViewport` _undertale_widget 0)))

(event `self.OnDeselected`
  (`Widget.SetVisibility` (`self.Undertale Widget`) "Collapsed")
  (`Widget.SetVisibility` (`/Game/UI/MissionControl/MissionControl_MainDialogue.MasterBox` (`self.Widget`)) "SelfHitTestInvisible")
  (`parent.OnDeselected`))

(fn `Break Sentence into Lines`
  (params (Sentence :type String))
  (returns (Lines :type "Array of String"))
  (locals (Length :type Integer) (String :type String) (`New Line` :type Boolean :default true) (Result :type "Array of String"))
  (bind _string (`local.String`))
  (for _array_element (`KismetStringLibrary.ParseIntoArray` Sentence " " false)
    (if (`local.New Line`)
      (set `local.New Line` false :!label _label)
      (bind _output_get (set `local.String` _array_element))
      (if (> (`KismetStringLibrary.Len` _output_get) (`self.Character Limit`)) :!label _label_2
        (`KismetArrayLibrary.Array_Add` (`local.Result`) (`KismetStringLibrary.GetSubstring` (`local.String`) 0 (`self.Character Limit`)))
        (set `local.String` (`KismetStringLibrary.RightChop` (`local.String`) 25))
        (goto _label_2))
      (else
        (bind _returnvalue (`KismetStringLibrary.Concat_StrStr` (`local.String`) " " _array_element))
        (if (> (`KismetStringLibrary.Len` _returnvalue) (`self.Character Limit`))
          (`KismetArrayLibrary.Array_Add` (`local.Result`) (`local.String`))
          (goto _label)
          (else
            (set `local.String` _returnvalue))))))
  (if (> (`KismetStringLibrary.Len` _string) 0)
    (`KismetArrayLibrary.Array_Add` (`local.Result`) _string))
  (return (`local.Result`)))

(fn `Break String into Sentences`
  (params (String :type String))
  (returns (Sentences :type "Array of String"))
  (locals (Punctuation :type String :default ".!?") (Start :type Integer) (End :type Integer) (Result :type "Array of String"))
  (bind _result (`local.Result`))
  (bind _start (`local.Start`))
  (bind _returnvalue (`KismetStringLibrary.Trim` (`KismetStringLibrary.RightChop` String (`local.Start`))))
  (for (_array_element _array_index) (`KismetStringLibrary.GetCharacterArrayFromString` String)
    (if (`KismetStringLibrary.Contains` (`local.Punctuation`) _array_element)
      (set `local.End` _array_index)
      (elif (> (`local.End`) (`local.Start`))
        (`KismetArrayLibrary.Array_Add` (`local.Result`) (`KismetStringLibrary.Trim` (`KismetStringLibrary.GetSubstring` String _start (+ (- (`local.End`) _start) 1))))
        (bind _output_get (set `local.End` _array_index))
        (set `local.Start` _output_get))))
  (if (> (`KismetStringLibrary.Len` _returnvalue) 0)
    (`KismetArrayLibrary.Array_Add` _result _returnvalue))
  (return _result))

(fn `Format String Into Lines`
  (params (String :type String))
  (returns (Lines :type "Array of String"))
  (locals (Result :type "Array of String"))
  (bind _returnvalue (mod (`KismetArrayLibrary.Array_Length` (`local.Result`)) 3))
  (for _array_element (`self.Break String into Sentences` String)
    (if (not (== _returnvalue 0))
      (bind _lines (`self.Break Sentence into Lines` _array_element))
      (if (not (<= (`KismetArrayLibrary.Array_Length` _lines) (- 3 _returnvalue)))
        (for _ (range _returnvalue)
          (`KismetArrayLibrary.Array_Add` (`local.Result`)))))
    (`KismetArrayLibrary.Array_Append` (`local.Result`) _lines))
  (return (`local.Result`)))

(fn `UserConstructionScript`
  (`parent.UserConstructionScript`))