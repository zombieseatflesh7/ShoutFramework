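; BP_DropPod_Base is a drop pod Blueprint whose graphs are almost entirely empty stubs.
; It declares hooks for drilling, impact, departure, doors, ramp, player entry and exit, and mule ("Donkey") loading and unloading.
; A few events, such as BeginPlay, overlaps, impact, drilling start and ramp replication, only forward to the parent.
; The remaining events and functions, including timelines and RepNotifies, do nothing or return empty or default values.
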(event `self.ReceiveBeginPlay`
  (`parent.ReceiveBeginPlay`))

(event `self.ReceiveActorBeginOverlap`
  (params (OtherActor :type "Actor Object Reference"))
  (`parent.ReceiveActorBeginOverlap` OtherActor))

(event `Timeline_5__FinishedFunc`)

(event `Timeline_5__UpdateFunc`)

(event `Timeline_1__FinishedFunc`)

(event `Timeline_1__UpdateFunc`)

(event `Timeline_0__FinishedFunc`)

(event `Timeline_0__UpdateFunc`)

(event `self.ReceiveActorEndOverlap`
  (params (OtherActor :type "Actor Object Reference"))
  (`parent.ReceiveActorEndOverlap` OtherActor))

(event `StartDeparture`)

(event `self.OnDroppodImpact`
  (`parent.OnDroppodImpact`))

(event `Start Donkey Unload Sequence`)

(event `Unload Donkey`)

(event `self.OnDrillingStarted`
  (`parent.OnDrillingStarted`))

(event `Load Donkey`
  (params (Mule :type "MULE Object Reference")))

(event `DrillRotate`)

(event `OnCharacterEnter`
  (params (Character :type "PlayerCharacter Object Reference")))

(event `OnCharacterExit`
  (params (Character :type "PlayerCharacter Object Reference")))

(event `DropPodSetAnsel`
  (params (Active :type Boolean)))

(event `AllSetAnsel`
  (params (Active :type Boolean)))

(event `MakeTruckerDicesMove`)

(event `OnFirstPlayerLeftPod`)

(event `self.ReceiveDestroyed`
  (`parent.ReceiveDestroyed`))

(event `OnRepDoorState`)

(event `LowerMuleToGround`)

(event `OpenMuleBay`)

(event `OnMuleBayOpenedDispatch_Event_0`)

(event `self.SetMuleInstance`
  (params (Donkey :type "Molly Object Reference"))
  (`parent.SetMuleInstance` Donkey))

(event `self.OnRep_RampState`
  (`parent.OnRep_RampState`))

(event `OnGeneratedMissionChanged`
  (params (OutGeneratedMission :type "GeneratedMission Object Reference")))

(fn `AnyPlayersOnRamp`
  (returns (ReturnValue :type Boolean))
  (return false))

(fn `CloseRamp`)

(fn `CollectMule`
  (params (Mule :type "MULE Object Reference")))

(fn `DestroyIfClose`
  (params (Actors :type "Array of Actor Object Reference (by ref)") (DistanceSQ :type "Float (double-precision)")))

(fn `EnableMulebay`)

(fn `GetCountDown`
  (params (First :type Boolean))
  (return))

(fn `GetDonkeyReturnPickupLocation`
  (returns (ReturnValue :type "Vector Structure"))
  (bind _returnvalue (`parent.GetDonkeyReturnPickupLocation`))
  (return _returnvalue))

(fn `GetMule`
  (returns (Donkey :type "Molly Object Reference"))
  (return null))

(fn `GetMuleUnloadTarget`
  (params (Mule :type "MULE Object Reference (by ref)"))
  (returns (RelativeTransform :type "Transform Structure"))
  (return))

(fn `HandleRampPhotosensitivity`)

(fn `OnAllPlayersLeftPod`)

(fn `OnMuleLoaded`)

(fn `OnRep_DoorState`)

(fn `OnRep_MuleInstance`)

(fn `OnRep_MuleSequenceComplete`)

(fn `OnRep_MuleUnloadTransform`)

(fn `OpenRamp`)

(fn `OperateMuleBay`
  (params (Open :type Boolean))
  (returns (ReturnValue :type "Float (double-precision)") (Montage :type "AnimMontage Object Reference"))
  (return 0.0 null))

(fn `RemoveDangerousCaveItems`
  (params (Distance :type "Float (double-precision)")))

(fn `SetAllPlayersAnsel`
  (params (Active :type Boolean)))

(fn `SetDoorState`
  (params (DoorState :type "/Game/Art/DropPod/DroppodDoorState Enum" :default "NewEnumerator0")))

(fn `SetPathBlockersEnabled`
  (params (Enable :type Boolean)))

(fn `SetPreferredCharacter`
  (params (Spawn :type "ChildActorComponent Object Reference") (Class :type "PlayerCharacterID Object Reference")))

(fn `SetStandingDown`
  (params (IsStandingDown :type Boolean)))

(fn `UserConstructionScript`)